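; Sailing boat Blueprint that turns keyboard input into steering and throttle values.
; Enables input from player controller 0 on BeginPlay, then arrow keys set SteeringInput left or right and Up sets a forward ThrottleInput, each resetting to zero on release.
; The graph only writes these values and prints a debug string for Up, with no movement logic of its own.
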(event `Key|Right`
  (params (Key :type "Key Structure"))
  (:`Pressed`
    (set `self.SteeringInput` 1.0))
  (:`Released`
    (set `self.SteeringInput` 0.0)))

(event `Key|Left`
  (params (Key :type "Key Structure"))
  (:`Pressed`
    (set `self.SteeringInput` -1.0))
  (:`Released`
    (set `self.SteeringInput` 0.0)))

(event `Key|Up`
  (params (Key :type "Key Structure"))
  (:`Pressed`
    (set `self.ThrottleInput` 0.5)
    (`KismetSystemLibrary.PrintString` "Up" :!label _label))
  (:`Released`
    (set `self.ThrottleInput` 0.0)
    (goto _label)))

(event `self.ReceiveBeginPlay`
  (`self.EnableInput` (`GameplayStatics.GetPlayerController` 0)))

(fn `UserConstructionScript`
  (`parent.UserConstructionScript`))