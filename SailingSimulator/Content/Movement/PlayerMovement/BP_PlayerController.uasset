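; Player controller Blueprint that handles Enhanced Input movement and camera look for the controlled pawn.
; BeginPlay adds the input mapping context to the local player subsystem.
; The camera action feeds yaw and pitch input.
; The move action pushes the pawn along the controller's own forward and right vectors rather than the pawn's, with action X driving forward and Y driving right.
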(event `EnhancedInput|/Game/Movement/PlayerMovement/AC_Camera`
  (params (ActionValue :type "Vector2D Structure") (ElapsedSeconds :type "Float (double-precision)") (TriggeredSeconds :type "Float (double-precision)") (InputAction :type "InputAction Object Reference" :default "/Game/Movement/PlayerMovement/AC_Camera.AC_Camera"))
  (bind (_x _y) (`KismetMathLibrary.BreakVector2D` ActionValue))
  (:`Triggered`
    (`self.AddYawInput` _x)
    (`self.AddPitchInput` _y)))

(event `EnhancedInput|/Game/Movement/PlayerMovement/AC_Move`
  (params (ActionValue :type "Vector2D Structure") (ElapsedSeconds :type "Float (double-precision)") (TriggeredSeconds :type "Float (double-precision)") (InputAction :type "InputAction Object Reference" :default "/Game/Movement/PlayerMovement/AC_Move.AC_Move"))
  (bind (_returnvalue_x _returnvalue_y _returnvalue_z) (`KismetMathLibrary.BreakVector` (`self.GetActorForwardVector`)))
  (bind (_returnvalue_x_2 _returnvalue_y_2 _returnvalue_z_2) (`KismetMathLibrary.BreakVector` (`self.GetActorRightVector`)))
  (bind (_x _y) (`KismetMathLibrary.BreakVector2D` ActionValue))
  (bind _returnvalue (`self.K2_GetPawn`))
  (:`Triggered`
    (`Pawn.AddMovementInput` _returnvalue (`KismetMathLibrary.MakeVector` _returnvalue_x_2 _returnvalue_y_2 _returnvalue_z_2) _y false)
    (`Pawn.AddMovementInput` _returnvalue (`KismetMathLibrary.MakeVector` _returnvalue_x _returnvalue_y _returnvalue_z) _x false)))

(event `self.ReceiveBeginPlay`
  (`EnhancedInputSubsystemInterface.AddMappingContext` (subsystem `EnhancedInputLocalPlayerSubsystem`) "/Game/Movement/PlayerMovement/InputMapping.InputMapping" 0 (struct)))

(fn `UserConstructionScript`)