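; WindController is a Blueprint that drives the ocean's wind parameters at runtime.
; Each Tick it eases current wind angle and speed toward target values with FInterpTo, treating the angle as a plain float without wraparound.
; It writes speed, a normalized strength and an angle-derived direction vector to the MPC_Ocean parameter collection.
; It also casts the ocean actor's water waves to GerstnerWaterWaves, but leaves the result unused.
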(event `self.ReceiveTick`
  (params (DeltaSeconds :type "Float (single-precision)"))
  (bind _output_get (set `self.CurrentWindAngle` (`KismetMathLibrary.FInterpTo` (`self.CurrentWindAngle`) (`self.TargetWindAngle`) DeltaSeconds 0.5)))
  (bind _output_get_2 (set `self.CurrentWindSpeed` (`KismetMathLibrary.FInterpTo` (`self.CurrentWindSpeed`) (`self.TargetWindSpeed`) DeltaSeconds 0.3)))
  (`KismetMaterialLibrary.SetScalarParameterValue` "/Game/materials/MPC_Ocean.MPC_Ocean" "WindSpeed" _output_get_2)
  (`KismetMaterialLibrary.SetScalarParameterValue` "/Game/materials/MPC_Ocean.MPC_Ocean" "WindStrength" (`KismetMathLibrary.SafeDivide` _output_get_2 100.0))
  (`KismetMaterialLibrary.SetVectorParameterValue` "/Game/materials/MPC_Ocean.MPC_Ocean" "WindDirection" (`KismetMathLibrary.Conv_VectorToLinearColor` (`KismetMathLibrary.MakeVector` (`KismetMathLibrary.DegCos` _output_get) (`KismetMathLibrary.DegSin` _output_get))))
  (cast `GerstnerWaterWaves` (`WaterBodyComponent.GetWaterWaves` (`WaterBody.WaterBodyComponent` (`self.OceanActor`)))))

(fn `UserConstructionScript`)